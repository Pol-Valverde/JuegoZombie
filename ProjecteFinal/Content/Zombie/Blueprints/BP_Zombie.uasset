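; Zombie enemy character that chases the first-person player, attacks in melee and drops coins when killed.
; On BeginPlay it caches the player, then loops between AIMoveTo pursuit and a delayed punch that deals damage if the player is still in range.
; RestarVida, meant to be called by projectiles, subtracts health and on death sets a Dying flag, spawns random coins, stops movement and destroys the actor after the animation.
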(event Custom|RestarVida
  (params (Damage :type Float%20%28double-precision%29))
  ;[1 1 1] Funcion que resta la vida del Zombie, se llama desde el proyectil
  (bind _output_get (Variables|Default|SetvidaZombie (- (Variables|Default|GetvidaZombie) Damage)))
  (if (<= _output_get 0.0)
    (if (not (Variables|Default|GetDying))
      (CallFunction|SpawnCoins)
      (Variables|Default|SetDying true)
      (Components|Animation|PlayAnimation (Variables|Character|GetMesh) "/Game/Zombie/Assets/Zombie_Dying.Zombie_Dying" false)
      (Variables|/Script/Engine.CharacterMovementComponent|SetMaxWalkSpeed (Variables|Character|GetCharacterMovement) 0.0)
      (Utilities|FlowControl|Delay 2.5)
      (Actor|DestroyActor))))

(event Custom|SeguirJugador
  ;[1 1 1] Seguir Jugador
  (Components|Animation|PlayAnimation (Variables|Character|GetMesh) "/Game/Zombie/Assets/Zombie_Run.Zombie_Run" true)
  (AI|AIMoveTo self "0, 0, 0" (Variables|Default|GetAs%20BP%20First%20Person%20Character) 5.0 false
    (:OnSuccess
      (CallFunction|Atacar))
    (:OnFail
      (CallFunction|SeguirJugador))))

(event Custom|Atacar
  ;[1 1 1] Ataque zombie
  (if (not (Variables|Default|GetDying))
    (Audio|PlaySoundatLocation "/Game/Zombie/Sonidos/ZombieSoundCue.ZombieSoundCue" (Transformation|GetWorldLocation (Variables|Character|GetMesh)) "0, 0, 0" 1.0 1.0 0.0 0 0 0 0)
    (Components|Animation|PlayAnimation (Variables|Character|GetMesh) "/Game/Zombie/Assets/Zombie_Punching.Zombie_Punching" false)
    (Utilities|FlowControl|Delay 1.0)
    (if (<= (Math|Vector|Distance(Vector) (Transformation|GetWorldLocation (Variables|Character|GetMesh)) (Transformation|GetWorldLocation (Variables|/Script/Engine.Character|GetMesh (Variables|Default|GetAs%20BP%20First%20Person%20Character)))) 2.5e+02)
      (Default|RecibirDanio (Variables|Default|GetAs%20BP%20First%20Person%20Character) (Variables|Default|GetDanioAtaque))
      (else
        (Development|PrintString "No he recibido daño")))
    (Utilities|FlowControl|Delay 1.0)
    (CallFunction|SeguirJugador)))

(event Custom|SpawnCoins
  (bind _mesh (Variables|Character|GetMesh))
  (bind _returnvalue (Transformation|GetWorldLocation _mesh))
  (for _index (range 0 (- (Math|Random|RandomIntegerinRange 1 3) 1))
    (Game|SpawnActorfromClass "/Game/Coins/BP_Coins.BP_Coins_C" (Math|Transform|MakeTransform (Math|Vector|MakeVector (+ (.x _returnvalue) (Math|Random|RandomFloatinRange -3e+01 3e+01)) (+ (.y _returnvalue) (Math|Random|RandomFloatinRange -3e+01 3e+01)) (.z _returnvalue)) "0, 0, 0" "1.000000,1.000000,1.000000") "Undefined" "MultiplyWithRoot" 0 0)))

(event EventBeginPlay
  ;[1 1 1] BeginPlay
  (bind _returnvalue (Actor|GetActorOfClass "/Game/FirstPerson/Blueprints/BP_FirstPersonCharacter.BP_FirstPersonCharacter_C"))
  (bind _asbp_first_person_character (Utilities|Casting|CastToBP_FirstPersonCharacter _returnvalue))
  (Variables|Default|SetAs%20BP%20First%20Person%20Character _asbp_first_person_character)
  (CallFunction|SeguirJugador))

(fn ConstructionScript)