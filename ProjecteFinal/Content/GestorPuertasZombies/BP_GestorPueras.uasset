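; BP_GestorPueras is a zombie door manager that spawns waves (oleadas) from the doors in its Puertas array.
; On BeginPlay, if IsOpened is true, it starts an endless delayed loop that requests waves without rechecking the flag.
; Each wave waits, calls SpawnZombie on every door, then recurses while decrementing NumeroDeZombies.
; The counter is never reset here, so once exhausted, later waves spawn once per door.
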(event Custom|SpawnOleada
  (Utilities|FlowControl|Delay 7.0)
  (for _array_element (Variables|Default|GetPuertas)
    (Default|SpawnZombie _array_element))
  (if (not (<= (Variables|Default|GetNumeroDeZombies) 0))
    (Variables|Default|SetNumeroDeZombies (- (Variables|Default|GetNumeroDeZombies) 1))
    (CallFunction|SpawnOleada)))

(event Custom|StartOleadas
  (if (Variables|Default|GetisOpened)
    (CallFunction|SpawnOleada :!label _label)
    (Utilities|FlowControl|Delay 3e+01)
    (goto _label)))

(event EventBeginPlay
  (CallFunction|StartOleadas))

(fn ConstructionScript)