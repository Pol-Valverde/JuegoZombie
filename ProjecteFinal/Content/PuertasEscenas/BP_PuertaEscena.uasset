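; BP_PuertaEscena is a coin-gated scene door that the player buys open by walking into its Box trigger.
; On overlap, it casts to BP_FirstPersonCharacter and, if enough Monedas are held, deducts the fixed price and passes the new total to the WICoins widget.
; It then flags GestorPuertas as opened, calls its StartOleadas to begin the waves, and destroys itself.
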(event OnComponentBeginOverlap(Box)
  (params (OverlappedComponent :type Primitive%20Component%20Object%20Reference) (OtherActor :type Actor%20Object%20Reference) (OtherComp :type Primitive%20Component%20Object%20Reference) (OtherBodyIndex :type Integer) (bFromSweep :type Boolean) (SweepResult :type Hit%20Result%20Structure%20%28by%20ref%29))
  (bind _asbp_first_person_character (Utilities|Casting|CastToBP_FirstPersonCharacter OtherActor))
  (if (>= (Variables|/Game/FirstPerson/Blueprints/BP_FirstPersonCharacter.BP_FirstPersonCharacter_C|GetMonedas _asbp_first_person_character) 30)
    (bind _output_get (Variables|/Game/FirstPerson/Blueprints/BP_FirstPersonCharacter.BP_FirstPersonCharacter_C|SetMonedas _asbp_first_person_character (- (Variables|/Game/FirstPerson/Blueprints/BP_FirstPersonCharacter.BP_FirstPersonCharacter_C|GetMonedas _asbp_first_person_character) 30)))
    (Default|IncrementValue (Variables|/Game/FirstPerson/Blueprints/BP_FirstPersonCharacter.BP_FirstPersonCharacter_C|GetWI_Coins _asbp_first_person_character) _output_get)
    (Variables|/Game/GestorPuertasZombies/BP_GestorPueras.BP_GestorPueras_C|SetisOpened (Variables|Default|GetGestorPuertas) true)
    (Default|StartOleadas (Variables|Default|GetGestorPuertas))
    (Actor|DestroyActor)))

(event EventBeginPlay)

(event Collision|EventActorBeginOverlap
  (params (OtherActor :type Actor%20Object%20Reference)))

(event EventTick
  (params (DeltaSeconds :type Float%20%28single-precision%29)))

(fn ConstructionScript)